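; Player controller that puts an on-screen console and its message widgets into the game.
; ShowConsoleWidget creates WBP_Console, adds it to the viewport and switches to game-and-UI input focused on it.
; The O key appends a WBP_ConsoleMessage to ConsoleMessageEntry's EntryBox, but the code creating that entry widget is disconnected.
; BeginPlay sets CanDisplayConsoleWidget, which this graph never reads.
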(event Custom|ShowConsoleWidget
  (bind _returnvalue (UserInterface|CreateWidget "/Game/UI/WBP_Console.WBP_Console_C" (Game|GetPlayerController 0)))
  (bind _output_get (Variables|Default|SetWBPConsole _returnvalue))
  (Utilities|IsValid _output_get
    (:Is%20Valid
      (UserInterface|Viewport|AddtoViewport _returnvalue 0)
      (Input|SetInputModeGameandUI (Game|GetPlayerController 0) _returnvalue "DoNotLock" true))))

(event EventBeginPlay
  (Variables|Default|SetCanDisplayConsoleWidget true))

(event EventTick
  (params (DeltaSeconds :type Float%20%28single-precision%29)))

(event Input|KeyboardEvents|O
  (params (Key :type Key%20Structure :default "None"))
  (:Pressed
    (bind _returnvalue (UserInterface|CreateWidget "/Game/UI/WBP_ConsoleMessage.WBP_ConsoleMessage_C" (Game|GetPlayerController 0)))
    (Widget|Panel|AddChild (Variables|/Game/UI/WBP_ConsoleMessageEntry.WBP_ConsoleMessageEntry_C|GetEntryBox (Variables|Default|GetConsoleMessageEntry)) _returnvalue)))

(fn ConstructionScript)